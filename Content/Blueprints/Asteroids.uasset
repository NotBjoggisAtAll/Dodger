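; An asteroid actor that drifts across the screen at a random speed while spinning.
; BeginPlay picks a negative fall speed and a roll rate, which Tick applies as a local X offset and rotation each frame, without delta-time scaling.
; Rolling about local X keeps the travel direction straight.
; The asteroid destroys itself when its static mesh ends overlap with an InvisibleWall at the screen's edge.
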(event OnComponentEndOverlap(StaticMesh)
  (params (OverlappedComponent :type Primitive%20Component%20Object%20Reference) (OtherActor :type Actor%20Object%20Reference) (OtherComp :type Primitive%20Component%20Object%20Reference) (OtherBodyIndex :type Integer))
  ;[0 0.5024 0.3189] Destroys the asteroid when it reaches the end of the screen
  (if (.bSuccess (Utilities|Casting|CastToInvisibleWall OtherActor))
    (Actor|DestroyActor)))

(event EventBeginPlay
  ;[0 0.2802 0.5411] BeginPlay
  ;;[0.3092 0 0.5182] Set Random Fallspeed
  (Variables|Default|SetFallSpeed (* (Math|Random|RandomFloatinRange 5.0 4e+01) -1.0))
  ;;[0.2319 0.5894 0] Set Random Rotation
  (Variables|Default|SetRotation (Math|Random|RandomFloatinRange -3.0 3.0)))

(event EventTick
  (params (DeltaSeconds :type Float%20%28single-precision%29))
  ;[0.3285 0 0.4987] Tick
  ;;[0.5508 0 0.2738] Adds Fallspeed and Rotation Every Tick
  (Transformation|AddActorLocalOffset (Math|Vector|MakeVector (Variables|Default|GetFallSpeed) 0.0 0.0) false false)
  (Transformation|AddActorLocalRotation (Math|Rotator|MakeRotator (Variables|Default|GetRotation) 0.0 0.0) false false))

(fn ConstructionScript)