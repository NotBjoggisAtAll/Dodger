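; LazerBeam is the player's laser shot actor, which destroys asteroids on impact and awards score.
; On BeginPlay it plays the shoot sound with a slightly randomized pitch.
; When its Cube hits an Asteroids actor, it destroys both actors, increments the Player pawn's score, and plays an explosion sound and randomly rotated particle effect scaled from the asteroid's size.
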(event OnComponentHit(Cube)
  (params (HitComponent :type Primitive%20Component%20Object%20Reference) (OtherActor :type Actor%20Object%20Reference) (OtherComp :type Primitive%20Component%20Object%20Reference) (NormalImpulse :type Vector :default "0, 0, 0") (Hit :type Hit%20Result%20Structure%20%28by%20ref%29))
  (bind (_asasteroids _bsuccess) (Utilities|Casting|CastToAsteroids OtherActor))
  (if _bsuccess
    (Actor|DestroyActor)
    (CallFunction|IncrementScore)
    ;[0.2416 0 0.5866] Spawn Particles
    (Effects|SpawnEmitteratLocation "/Game/P_Explosion.P_Explosion" (Transformation|GetActorLocation) (Math|Random|RandomRotator false) (- (Transformation|GetActorScale3D _asasteroids) 1.5))
    (Actor|DestroyActor _asasteroids)
    (Audio|PlaySound2D "/Game/Sounds/AsteroidSound.AsteroidSound" 1.0 1.0 0.0 0 0)))

(event EventBeginPlay
  ;[0.02899 0.7923 0] Play LazerBeam Sound at BeginPlay
  (Audio|PlaySound2D "/Game/Sounds/PlayerShootSound.PlayerShootSound" 1.0 (Math|Random|RandomFloatinRange 0.9 1.1) 0.0 0 0))

(fn ConstructionScript)

(fn IncrementScore
  (bind _returnvalue (Game|Player|GetPlayerPawn 0))
  (bind (_asplayer _bsuccess) (Utilities|Casting|CastToPlayer _returnvalue))
  (if _bsuccess
    (bind _result (Math|Integer|IncrementInt (Class|Ship|GetScore _asplayer))
      (:%20%20
        (Class|Ship|SetScore _asplayer _result)))))