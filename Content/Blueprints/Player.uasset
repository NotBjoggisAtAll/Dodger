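; Player actor for a shooter game that fires lasers and records the high score when destroyed.
; Shoot input spawns a scaled LazerBeam at a fixed world X offset, with a CanFire flag and Delay limiting fire rate.
; On Destroyed, it loads or creates the "scores" save and stores ShooterGameMode's current score if it beats the saved high score.
; A swept local-offset movement node exists but never runs.
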(event EventDestroyed
  (bind _returnvalue (Game|GetGameMode))
  (bind (_asshooter_game_mode _bsuccess) (Utilities|Casting|CastToShooterGameMode _returnvalue))
  (bind _currentscore (Variables|/Game/Blueprints/ShooterGameMode.ShooterGameMode_C|GetCurrentScore _asshooter_game_mode))
  (if _bsuccess
    (bind _returnvalue_2 (SaveGame|LoadGamefromSlot "scores"))
    (bind _asmy_save (Utilities|Casting|CastToMySave _returnvalue_2)
      (:then
        _)
      (:CastFailed
        (SaveGame|CreateSaveGameObject "/Game/Blueprints/MySave.MySave_C")))
    (if true
      (if (> _currentscore (Variables|/Game/Blueprints/MySave.MySave_C|GetHighScore _asmy_save))
        (bind _output_get (Variables|/Game/Blueprints/ShooterGameMode.ShooterGameMode_C|SetHighScore _asshooter_game_mode _currentscore))
        (Variables|/Game/Blueprints/MySave.MySave_C|SetHighScore _asmy_save _output_get)
        (SaveGame|SaveGametoSlot _asmy_save "scores")))))

(event Input|ActionEvents|InputActionShoot
  (params (Key :type Key%20Structure))
  ;[0 0.2705 0.5508] Shoot
  (:Pressed
    (if (Variables|Default|GetCanFire)
      (Variables|Default|SetCanFire false)
      (Game|SpawnActorfromClass "/Game/Blueprints/LazerBeam.LazerBeam_C" (Math|Transform|MakeTransform (+ (Transformation|GetActorLocation) "400.000000,0.000000, 0") (Transformation|GetActorRotation) "0.800000,0.200000,0.200000") "AdjustIfPossibleButAlwaysSpawn" 0 0)
      (Utilities|FlowControl|Delay (Variables|Default|GetFireRate))
      (Variables|Default|SetCanFire true))))

(fn ConstructionScript)